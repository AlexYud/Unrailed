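; Interactable hinged door that the player swings open or closed, optionally allowing repeated use.
; A timeline scaled by OpeningTime rotates the hinge yaw through a quarter turn, playing forward to open and in reverse to close.
; If the player overlaps StopCollision during the swing, the timeline changes direction and the door becomes interactable again when it finishes.
; A proximity volume shows or hides the interaction icon widget, which also reflects focus.
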(event `self.ReceiveBeginPlay`
  (`self.BeginPlayGetRefs`))

(event `/Game/Unrailed/Blueprints/Interfaces/Interactable.Interact`
  (set `self.Can_Interact` false)
  (set `self.Cancelled` false)
  (`self.Open / Close`))

(event `Open / Close`
  (`TimelineComponent.SetPlayRate` (`self.Open/Close_TL`) (/ 1.0 (`self.OpeningTime`)))
  (if (not (`self.IsOpen`))
    (bind (_direction _newtrack_0) (`Timeline|Open/Close_TL` :!via `PlayFromStart` :!label _label)
      (:`Update`
        (`SceneComponent.K2_SetRelativeRotation` (`self.Hinge`) (`KismetMathLibrary.MakeRotator` 0.0 0.0 (`KismetMathLibrary.Lerp` 0.0 -90.0 _newtrack_0)) false false)
        (if (`PrimitiveComponent.IsOverlappingActor` (`self.StopCollision`) (`GameplayStatics.GetPlayerCharacter` 0))
          (`self.CancelMovement`)
          (set `self.Cancelled` true)))
      (:`Finished`
        (switch `ETimelineDirection` _direction
          (:`Forward`
            (set `self.IsOpen` true))
          (:`Backward`
            (set `self.IsOpen` false)))
        (if (or (`self.ReInteractable`) (`self.Cancelled`))
          (set `self.Can_Interact` true))))
    (else
      (goto _label :!via `ReverseFromEnd`))))

(event `CancelMovement`
  (bind _open_close_tl (`self.Open/Close_TL`))
  (if (`TimelineComponent.IsPlaying` _open_close_tl)
    (if (`TimelineComponent.IsReversing` _open_close_tl)
      (`TimelineComponent.Play` _open_close_tl)
      (else
        (`TimelineComponent.Reverse` _open_close_tl)))))

(event `self.InteractionIconShowCollision.OnComponentBeginOverlap`
  (params (OverlappedComponent :type "PrimitiveComponent Object Reference") (OtherActor :type "Actor Object Reference") (OtherComp :type "PrimitiveComponent Object Reference") (OtherBodyIndex :type Integer) (bFromSweep :type Boolean) (SweepResult :type "HitResult Structure (by ref)"))
  (cast `/Game/Unrailed/Blueprints/BP_Player_Character` OtherActor)
  (`/Game/Unrailed/Blueprints/HUD/W_Interaction_Icon.Show / Hide` (`self.InteractIconWidgetRef`) true))

(event `self.InteractionIconShowCollision.OnComponentEndOverlap`
  (params (OverlappedComponent :type "PrimitiveComponent Object Reference") (OtherActor :type "Actor Object Reference") (OtherComp :type "PrimitiveComponent Object Reference") (OtherBodyIndex :type Integer))
  (cast `/Game/Unrailed/Blueprints/BP_Player_Character` OtherActor)
  (`/Game/Unrailed/Blueprints/HUD/W_Interaction_Icon.Show / Hide` (`self.InteractIconWidgetRef`) false))

(event `/Game/Unrailed/Blueprints/Interfaces/Interactable.Set_Focus`
  (params (Focus :type Boolean))
  (`/Game/Unrailed/Blueprints/HUD/W_Interaction_Icon.Set_Focus` (`self.InteractIconWidgetRef`) Focus))

(fn `BeginPlayGetRefs`
  (bind _asw_interaction_icon (cast `/Game/Unrailed/Blueprints/HUD/W_Interaction_Icon` (`WidgetComponent.GetWidget` (`self.InteractIcon`))))
  (set `self.InteractIconWidgetRef` _asw_interaction_icon))

(fn `CanInteract`
  (returns (Result :type Boolean))
  (return (`self.Can_Interact`)))

(fn `UserConstructionScript`)